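; BP_Door is an interactable hinged door for the school challenge that registers itself with GI_Main on BeginPlay.
; Interact, OpenDoor and CloseDoor feed a shared animation event that, unless locked, runs a duration-scaled timeline forward or in reverse to lerp the pivot's rotation.
; The first Interact plays an opening sound, even if locked.
; A one-shot trigger box closes and locks the door on overlap, then destroys itself.
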(event `self.ReceiveBeginPlay`
  (bind _asgi_main (cast `/Game/BPs/Game/GI_Main` (`GameplayStatics.GetGameInstance`)))
  (set `/Game/BPs/Game/GI_Main.Door` self _asgi_main)
  (set `self.IsFirstOpen` true))

(event `CE_DoorAnim`
  (if (not (`self.IsLocked`))
    (`TimelineComponent.SetPlayRate` (`self.TL_DoorAnim`) (/ 1.0 (`self.DoorAnimDuration`)))
    (if (`self.IsOpen`)
      (`|ExecutionSequence`
        (:`then_0`
          (bind (_direction _weight) (`Timeline|TL_DoorAnim` :!via `ReverseFromEnd` :!label _label)
            (:`Update`
              (`SceneComponent.K2_SetRelativeRotation` (`self.pivot`) (`KismetMathLibrary.RLerp` (`self.CloseRotation`) (`self.OpenRotation`) _weight true) false false))))
        (:`then_1`
          (set `self.IsOpen` (not (`self.IsOpen`)) :!label _label_2)))
      (else
        (`|ExecutionSequence`
          (:`then_0`
            (goto _label :!via `PlayFromStart`))
          (:`then_1`
            (goto _label_2)))))))

(event `/Game/BPs/Interfaces/BPI_Interactible.Interact`
  (params (Component :type "ActorComponent Object Reference"))
  (`self.CE_DoorAnim`)
  (if (`self.IsFirstOpen`)
    (set `self.IsFirstOpen` false)
    (`GameplayStatics.PlaySound2D` "/Game/Assets/Sounds/MetaSounds/Voices/MS_SchoolDoorOpen.MS_SchoolDoorOpen" 1.0 1.0 0.0 null null)))

(event `self.Box.OnComponentBeginOverlap`
  (params (OverlappedComponent :type "PrimitiveComponent Object Reference") (OtherActor :type "Actor Object Reference") (OtherComp :type "PrimitiveComponent Object Reference") (OtherBodyIndex :type Integer) (bFromSweep :type Boolean) (SweepResult :type "HitResult Structure (by ref)"))
  (`self.CloseDoor`)
  (set `self.IsLocked` true)
  (`ActorComponent.K2_DestroyComponent` (`self.Box`)))

(fn `CloseDoor`
  (if (`self.IsOpen`)
    (`self.CE_DoorAnim`)))

(fn `OpenDoor`
  (if (not (`self.IsOpen`))
    (`self.CE_DoorAnim`)))

(fn `UserConstructionScript`)