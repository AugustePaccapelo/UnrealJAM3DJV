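; BP_Chair is an interactable chair for the school challenge that seats the player and completes the current level when they get up.
; Interact saves the pawn's transform, flags Chara_Player as sitting with a chair reference, and snaps pawn and view to PlayerSitPos.
; Tick pins the player to the seat until IsSitted clears.
; GetUp restores the saved transform and view, then tells GI_Main to complete the level.
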(event `self.ReceiveTick`
  (params (DeltaSeconds :type "Float (single-precision)"))
  (bind _player (`self.Player`)
    (:`then`
      (if (`/Game/BPs/Player/Chara_Player.IsSitted` _player)
        (`self.K2_SetActorLocation` (`self.Player`) (`SceneComponent.K2_GetComponentLocation` (`self.PlayerSitPos`)) false false)
        (else
          (set `self.Player` null))))
    (:`else`)))

(event `/Game/BPs/Interfaces/BPI_Interactible.Interact`
  (bind _returnvalue (`GameplayStatics.GetPlayerPawn` 0))
  (bind _returnvalue_2 (`SceneComponent.K2_GetComponentToWorld` (`self.PlayerSitPos`)))
  (set `self.BasePlayerTransform` (`self.GetTransform` _returnvalue))
  (bind _aschara_player (cast `/Game/BPs/Player/Chara_Player` _returnvalue))
  (set `self.Player` _aschara_player)
  (set `/Game/BPs/Player/Chara_Player.IsSitted` true _aschara_player)
  (set `/Game/BPs/Player/Chara_Player.Chair` self _aschara_player)
  (`self.K2_SetActorTransform` _returnvalue _returnvalue_2 false false)
  (`Controller.SetControlRotation` (`Pawn.GetController` _returnvalue) (.rotation _returnvalue_2)))

(fn `GetUp`
  (bind _returnvalue (`GameplayStatics.GetPlayerPawn` 0))
  (bind _baseplayertransform (`self.BasePlayerTransform`))
  (`self.K2_SetActorTransform` _returnvalue _baseplayertransform false false)
  (`Controller.SetControlRotation` (`Pawn.GetController` _returnvalue) (.rotation _baseplayertransform))
  (bind _asgi_main (cast `/Game/BPs/Game/GI_Main` (`GameplayStatics.GetGameInstance`)))
  (`/Game/BPs/Game/GI_Main.CompleteCurrentLevel` _asgi_main))

(fn `UserConstructionScript`)