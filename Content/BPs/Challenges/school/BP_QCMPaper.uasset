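; BP_QCMPaper is a multiple-choice (QCM) paper actor for the school challenge, with a WBP_QCMPage widget on its front and back.
; On BeginPlay it binds both pages' all-checked events to a page-finished handler.
; When either page finishes, both reset and a timeline lerps the actor's rotation through a 180-degree roll to turn the sheet over, with play rate derived from AnimDuration.
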(event `self.ReceiveBeginPlay`
  (bind _aswbp_qcmpage (cast `/Game/BPs/Challenges/school/WBP_QCMPage` (`WidgetComponent.GetWidget` (`self.RectoWidget`))))
  (bind _output_get (set `self.RectoWBP` _aswbp_qcmpage))
  (add `/Game/BPs/Challenges/school/WBP_QCMPage.ED_OnAllChecked` _output_get (delegate `proxy_OnPageFinished`))
  (bind _aswbp_qcmpage_2 (cast `/Game/BPs/Challenges/school/WBP_QCMPage` (`WidgetComponent.GetWidget` (`self.VersoWidget`))))
  (bind _output_get_2 (set `self.VersoWBP` _aswbp_qcmpage_2))
  (add `/Game/BPs/Challenges/school/WBP_QCMPage.ED_OnAllChecked` _output_get_2 (delegate `proxy_OnPageFinished`)))

(event `proxy_OnPageFinished`
  (`self.ce_TurnPage`))

(event `ce_TurnPage`
  (`/Game/BPs/Challenges/school/WBP_QCMPage.Reset` (`self.RectoWBP`))
  (`/Game/BPs/Challenges/school/WBP_QCMPage.Reset` (`self.VersoWBP`))
  (`TimelineComponent.SetPlayRate` (`self.TurnTimeLine`) (/ 1.0 (`self.AnimDuration`)))
  (bind _output_get (set `self.StartRotator` (`self.K2_GetActorRotation`)))
  (set `self.EndRotator` (`KismetMathLibrary.MakeRotator` (+ (.roll _output_get) 180.0) (.pitch _output_get) (.yaw _output_get)))
  (bind (_direction _weight) (`Timeline|TurnTimeLine` :!via `PlayFromStart`)
    (:`Update`
      (`self.K2_SetActorRotation` (`KismetMathLibrary.RLerp` (`self.StartRotator`) (`self.EndRotator`) _weight)))))

(fn `UserConstructionScript`)