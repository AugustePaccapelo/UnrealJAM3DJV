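; BP_Socle is the moon challenge's pedestal, which completes the level when the player interacts while holding the light ball.
; It moves the ball onto BallPos, locks it against pickup and notifies GI_Main.
; A HUD fade then covers teleporting the player to the LightBall's starting transform before the OpenSas sequence plays.
; It also runs the moon background music and periodic monster sound on looping timers.
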(event `self.ReceiveBeginPlay`
  (bind _asgi_main (cast `/Game/BPs/Game/GI_Main` (`GameplayStatics.GetGameInstance`)))
  (set `self.GIMain` _asgi_main)
  (`GameplayStatics.PlaySound2D` "/Game/Assets/Sounds/MetaSounds/MS_MoonBackground.MS_MoonBackground" 4.0 1.0 0.0 null null)
  (`KismetSystemLibrary.K2_SetTimerDelegate` (delegate `proxy_SoundTimer`) 285.0 true)
  (`KismetSystemLibrary.K2_SetTimerDelegate` (delegate `proxy_MonsterSound`) (`self.TimeBetweenSounds`) true)
  (set `self.Teleport` (`self.GetTransform` (`self.LightBall`))))

(event `proxy_SoundTimer`
  (`GameplayStatics.PlaySound2D` "/Game/Assets/Sounds/MetaSounds/MS_MoonBackground.MS_MoonBackground" 4.0 1.0 0.0 null null))

(event `proxy_MonsterSound`
  (`GameplayStatics.PlaySoundAtLocation` "/Game/Assets/Sounds/MetaSounds/MS_MoonMonster.MS_MoonMonster" (`self.K2_GetActorLocation`) (struct) 1.0 1.0 0.0 null null self null))

(event `/Game/BPs/Interfaces/BPI_Interactible.Interact`
  (params (Component :type "ActorComponent Object Reference"))
  (bind _aschara_player (cast `/Game/BPs/Player/Chara_Player` (`GameplayStatics.GetPlayerPawn` 0)))
  (if (== (`GameplayStatics.GetObjectClass` (`/Game/BPs/Player/Chara_Player.ActorInHand` _aschara_player)) "/Game/BPs/Challenges/moon/BP_LightBall.BP_LightBall_C")
    (bind _actor (`/Game/BPs/Player/Chara_Player.RemoveActorInHand` _aschara_player))
    (`/Engine/EditorBlueprintResources/StandardMacros.IsValid` _actor
      (:`Is Valid`
        (`self.K2_SetActorTransform` _actor (`SceneComponent.K2_GetComponentToWorld` (`self.BallPos`)) false false)
        (bind _asbp_light_ball (cast `/Game/BPs/Challenges/moon/BP_LightBall` _actor))
        (set `/Game/BPs/Challenges/moon/BP_LightBall.CanBePicked` false _asbp_light_ball)
        (`/Game/BPs/Game/GI_Main.CompleteCurrentLevel` (`self.GIMain`))
        (bind _fondu (`/Game/BPs/Game/HUD_Game.Fondu` (`/Game/BPs/Player/Chara_Player.As HUD Game` _aschara_player)))
        (`TimelineComponent.PlayFromStart` _fondu)
        (`KismetSystemLibrary.Delay` 1.0)
        (`self.K2_SetActorTransform` (`GameplayStatics.GetPlayerPawn` 0) (`self.Teleport`) false false)
        (`TimelineComponent.ReverseFromEnd` _fondu)
        (`MovieSceneSequencePlayer.Play` (`LevelSequenceActor.SequencePlayer` (`self.OpenSas`)))))))

(fn `UserConstructionScript`)