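; Trigger volume for the main room that tracks whether the player is inside and handles the return from a completed level.
; Entering with a loaded, completed level plays a closing sequence, adding a school-end sound for one specific level, then unloads the level through GI_Main when the sequence finishes.
; The player snaps back to the start position when leaving with no level loaded, or when GI_Main's CanRedraw event fires while outside.
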(event `self.ReceiveBeginPlay`
  (bind _asgi_main (cast `/Game/BPs/Game/GI_Main` (`GameplayStatics.GetGameInstance`)))
  (bind _output_get (set `self.GIMain` _asgi_main))
  (add `/Game/BPs/Game/GI_Main.ED_CanRedraw` _output_get (delegate `ED_CanRedraw_Event`))
  (set `self.PlayerStartPos` (`self.K2_GetActorLocation` (`GameplayStatics.GetPlayerPawn` 0))))

(event `ED_CanRedraw_Event`
  (if (not (`self.IsPlayerInside`))
    (`self.K2_SetActorLocation` (`GameplayStatics.GetPlayerPawn` 0) (`self.PlayerStartPos`) false false)))

(event `self.Box.OnComponentBeginOverlap`
  (params (OverlappedComponent :type "PrimitiveComponent Object Reference") (OtherActor :type "Actor Object Reference") (OtherComp :type "PrimitiveComponent Object Reference") (OtherBodyIndex :type Integer) (bFromSweep :type Boolean) (SweepResult :type "HitResult Structure (by ref)"))
  (bind _gimain (`self.GIMain`))
  (bind _sequenceplayer (`LevelSequenceActor.SequencePlayer` (`self.SequenceClosing`)))
  (if (== (`GameplayStatics.GetObjectClass` OtherActor) "/Game/BPs/Player/Chara_Player.Chara_Player_C")
    (set `self.IsPlayerInside` true)
    (if (and (`/Game/BPs/Game/GI_Main.IsLevelComplete` _gimain) (`/Game/BPs/Game/GI_Main.IsALevelLoaded` _gimain))
      (`MovieSceneSequencePlayer.Play` _sequenceplayer)
      (add `MovieSceneSequencePlayer.OnFinished` _sequenceplayer (delegate `OnFinished_Event`))
      (if (`|EnumEquality` (`/Game/BPs/Game/GI_Main.CurrentLevel` _gimain) "NewEnumerator2")
        (`GameplayStatics.PlaySound2D` "/Game/Assets/Sounds/MetaSounds/Voices/MS_EndSchool.MS_EndSchool" 1.0 1.0 0.0 null null)))))

(event `OnFinished_Event`
  (`/Game/BPs/Game/GI_Main.UnloadCurrentLevel` (`self.GIMain`)))

(event `self.Box.OnComponentEndOverlap`
  (params (OverlappedComponent :type "PrimitiveComponent Object Reference") (OtherActor :type "Actor Object Reference") (OtherComp :type "PrimitiveComponent Object Reference") (OtherBodyIndex :type Integer))
  (if (== (`GameplayStatics.GetObjectClass` OtherActor) "/Game/BPs/Player/Chara_Player.Chara_Player_C")
    (if (`/Game/BPs/Game/GI_Main.IsALevelLoaded` (`self.GIMain`))
      (set `self.IsPlayerInside` false)
      (else
        (`self.K2_SetActorLocation` (`GameplayStatics.GetPlayerPawn` 0) (`self.PlayerStartPos`) false false)))))

(fn `UserConstructionScript`)