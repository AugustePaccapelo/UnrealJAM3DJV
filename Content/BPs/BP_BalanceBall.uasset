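; BP_BalanceBall is an actor that rolls forward by itself, moving along its arrow each tick while spinning its sphere mesh to match Speed.
; Each tick also has a small random chance to pick a left or right yaw offset and play the Rotation timeline, which lerps toward it.
; A DoOnce with no reset limits this turn to one occurrence.
; The timer that would drive the TimeVar counter is unconnected.
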(event `self.ReceiveBeginPlay`)

(event `Time`
  (`/Engine/EditorBlueprintResources/StandardMacros.IncrementFloat` (`self.TimeVar`)))

(event `self.ReceiveTick`
  (params (DeltaSeconds :type "Float (single-precision)"))
  (`self.RotateBall` DeltaSeconds)
  (`self.MoveBall`))

(fn `MoveBall`
  (`self.K2_SetActorLocation` (+ (* (`self.Speed`) (`SceneComponent.GetForwardVector` (`self.Arrow`))) (`self.K2_GetActorLocation`)))
  (`SceneComponent.K2_AddLocalRotation` (`self.Sphere`) (`KismetMathLibrary.MakeRotator` 0.0 (* (`self.Speed`) -1)) false false)
  (return))

(fn `RotateBall`
  (params (DeltaSeconds :type "Float (double-precision)"))
  (bind (_returnvalue_roll _returnvalue_pitch _returnvalue_yaw) (`KismetMathLibrary.BreakRotator` (`self.K2_GetActorRotation`)))
  (bind (_returnvalue_roll_2 _returnvalue_pitch_2 _returnvalue_yaw_2) (`KismetMathLibrary.BreakRotator` (`self.K2_GetActorRotation`)))
  (if (`KismetMathLibrary.RandomBoolWithWeight` 0.01)
    (`/Engine/EditorBlueprintResources/StandardMacros.DoOnce` false
      (:`Completed`
        (if (`KismetMathLibrary.RandomBoolWithWeight` 0.5)
          (set `self.TargetRot` (+ _returnvalue_yaw_2 (* (`KismetMathLibrary.RandomIntegerInRange` 1 3) 10)))
          (else
            (set `self.TargetRot` (+ _returnvalue_yaw (* (`KismetMathLibrary.RandomIntegerInRange` -3 -1) 10)))))
        (`TimelineComponent.PlayFromStart` (`self.Rotation`))
        (`KismetSystemLibrary.PrintString` "Hello")))
    (else
      (return))))

(fn `UserConstructionScript`)