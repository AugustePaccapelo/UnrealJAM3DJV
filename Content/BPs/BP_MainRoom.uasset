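; BP_MainRoom is the main room actor, which unloads the current level when the player enters it after that level is complete.
; It caches the GI_Main game instance on BeginPlay.
; Its Box overlap events track IsPlayerInside for Chara_Player, and on entry call UnloadCurrentLevel on GI_Main if IsLevelComplete is set.
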(event `self.ReceiveBeginPlay`
  (bind _asgi_main (cast `/Game/BPs/Game/GI_Main` (`GameplayStatics.GetGameInstance`)))
  (set `self.GIMain` _asgi_main))

(event `self.Box.OnComponentBeginOverlap`
  (params (OverlappedComponent :type "PrimitiveComponent Object Reference") (OtherActor :type "Actor Object Reference") (OtherComp :type "PrimitiveComponent Object Reference") (OtherBodyIndex :type Integer) (bFromSweep :type Boolean) (SweepResult :type "HitResult Structure (by ref)"))
  (bind _gimain (`self.GIMain`))
  (if (== (`GameplayStatics.GetObjectClass` OtherActor) "/Game/BPs/Player/Chara_Player.Chara_Player_C")
    (set `self.IsPlayerInside` true)
    (if (`/Game/BPs/Game/GI_Main.IsLevelComplete` _gimain)
      (`/Game/BPs/Game/GI_Main.UnloadCurrentLevel` _gimain))))

(event `self.Box.OnComponentEndOverlap`
  (params (OverlappedComponent :type "PrimitiveComponent Object Reference") (OtherActor :type "Actor Object Reference") (OtherComp :type "PrimitiveComponent Object Reference") (OtherBodyIndex :type Integer))
  (if (== (`GameplayStatics.GetObjectClass` OtherActor) "/Game/BPs/Player/Chara_Player.Chara_Player_C")
    (set `self.IsPlayerInside` false)))

(fn `UserConstructionScript`)