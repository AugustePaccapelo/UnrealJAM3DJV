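; BP_Card is a card actor that flies up to the camera, signals a room to open, then burns away.
; Init sets the front texture and text, then starts a timeline toward a camera-facing point cached at BeginPlay, while streaming in GI_Main's current level.
; On arrival it tracks the player, fires the OpenRoom dispatcher after a delay, later animates a material burn alongside a heterogeneous volume effect, and destroys itself.
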(event `self.ReceiveBeginPlay`
  (bind _returnvalue (`GameplayStatics.GetPlayerCameraManager` 0))
  (bind _front (`self.Front`))
  (bind _returnvalue_2 (`PlayerCameraManager.GetCameraLocation` _returnvalue))
  (bind (_returnvalue_roll _returnvalue_pitch _returnvalue_yaw) (`KismetMathLibrary.BreakRotator` (`PlayerCameraManager.GetCameraRotation` _returnvalue)))
  (bind _returnvalue_3 (+ _returnvalue_2 (* (`KismetMathLibrary.GetForwardVector` (`KismetMathLibrary.MakeRotator` 0.0 0.0 _returnvalue_yaw)) (`self.CardDistanceToCamera`))))
  (set `self.StartTransform` (`self.GetTransform`))
  (set `self.EndTransform` (`KismetMathLibrary.MakeTransform` _returnvalue_3 (`KismetMathLibrary.FindLookAtRotation` _returnvalue_3 _returnvalue_2)))
  (`SceneComponent.SetHiddenInGame` (`self.HeterogeneousVolume`) true false)
  (bind _returnvalue_4 (`PrimitiveComponent.CreateDynamicMaterialInstance` _front 0 (`PrimitiveComponent.GetMaterial` _front 0) "None"))
  (set `self.Mat` _returnvalue_4)
  (`KismetSystemLibrary.DelayUntilNextTick`)
  (`MaterialInstanceDynamic.SetTextureParameterValue` (`self.Mat`) "MainTexture" (`self.CardFront`)))

(event `self.ReceiveTick`
  (params (DeltaSeconds :type "Float (single-precision)"))
  (if (`self.LookAtPlayer`)
    (`self.K2_SetActorRotation` (`KismetMathLibrary.FindLookAtRotation` (`self.K2_GetActorLocation`) (`self.K2_GetActorLocation` (`GameplayStatics.GetPlayerPawn` 0))))))

(event `proxy_StartTL`
  (`TimelineComponent.SetPlayRate` (`self.TL_Spawn`) (/ 1.0 (`self.SpawnDuration`)))
  (`|ExecutionSequence`
    (:`then_0`
      (bind (_direction _weight) (`Timeline|TL_Spawn` :!via `PlayFromStart`)
        (:`Update`
          (`self.K2_SetActorTransform` (`KismetMathLibrary.TLerp` (`self.StartTransform`) (`self.EndTransform`) _weight)))
        (:`Finished`
          (set `self.LookAtPlayer` true)
          (`KismetSystemLibrary.Delay` (`self.WaitForOpenRoom`))
          (`self.ED_OpenRoom`)
          (`KismetSystemLibrary.Delay` (`self.DestroyAfterSeconds`))
          (`|ExecutionSequence`
            (:`then_0`
              (`TimelineComponent.SetPlayRate` (`self.TL_Burn`) (/ 1.0 (`self.BurnAnimDuration`)))
              (bind (_direction_2 _weight_2) (`Timeline|TL_Burn` :!via `PlayFromStart`)
                (:`Update`
                  (`MaterialInstanceDynamic.SetScalarParameterValue` (`self.Mat`) "Param" _weight_2))))
            (:`then_1`
              (`HeterogeneousVolumeComponent.SetPlaying` (`self.HeterogeneousVolume`) true)
              (`SceneComponent.SetHiddenInGame` (`self.HeterogeneousVolume`) false false)
              (`KismetSystemLibrary.Delay` (`self.BurnAnimDuration`))
              (`self.K2_DestroyActor`))))))
    (:`then_1`
      (bind _asgi_main (cast `/Game/BPs/Game/GI_Main` (`GameplayStatics.GetGameInstance`)))
      (bind (_value _returnvalue) (`BlueprintMapLibrary.Map_Find` (`/Game/BPs/Game/GI_Main.AllLevelsMap` _asgi_main) (`/Game/BPs/Game/GI_Main.CurrentLevel` _asgi_main)))
      (if _returnvalue
        (`GameplayStatics.LoadStreamLevel` _value true)))))

(fn `Init`
  (params (Text :type Text) (Texture :type "Texture Object Reference"))
  (bind _output_get (set `self.CardFront` Texture))
  (`MaterialInstanceDynamic.SetTextureParameterValue` (`self.Mat`) "MainTexture" _output_get)
  (`TextRenderComponent.K2_SetText` (`self.TextRender`) Text)
  (`self.proxy_StartTL`))

(fn `UserConstructionScript`)