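; Interactable card deck that draws the next level's card and, through that card, triggers the room-opening sequence.
; Construction stacks two instanced meshes, one flipped, and BeginPlay randomly jitters their rotations.
; Interact looks up GI_Main's next level in its data table, starts the level and spawns BP_Card from the top, with circus audio for one level.
; Drawing locks until GI_Main's redraw event; the card's open-room event plays the sequence and resets both smoke volumes.
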(event `proxy_CanRedraw`
  (set `self.CanDrawCard` true))

(event `self.ReceiveBeginPlay`
  (bind _instancedstaticmesh (`self.InstancedStaticMesh`))
  (bind (_cardsrandomrotations_roll _cardsrandomrotations_pitch _cardsrandomrotations_yaw) (`KismetMathLibrary.BreakRotator` (`self.CardsRandomRotations`)))
  (bind _returnvalue (* _cardsrandomrotations_yaw (`KismetMathLibrary.RandomFloatInRange` -1.0 1.0)))
  (bind _returnvalue_2 (* _cardsrandomrotations_roll (`KismetMathLibrary.RandomFloatInRange` -1.0 1.0)))
  (bind _returnvalue_3 (* _cardsrandomrotations_pitch (`KismetMathLibrary.RandomFloatInRange` -1.0 1.0)))
  (bind _asgi_main (cast `/Game/BPs/Game/GI_Main` (`GameplayStatics.GetGameInstance`)))
  (bind _output_get (set `self.As GI Main` _asgi_main))
  (add `/Game/BPs/Game/GI_Main.ED_CanRedraw` _output_get (delegate `proxy_CanRedraw`))
  (for _index (range (`InstancedStaticMeshComponent.GetInstanceCount` (`self.InstancedStaticMesh`)))
    (bind _outinstancetransform (`InstancedStaticMeshComponent.GetInstanceTransform` _instancedstaticmesh _index false))
    (`InstancedStaticMeshComponent.UpdateInstanceTransform` _instancedstaticmesh _index (`KismetMathLibrary.MakeTransform` (.location _outinstancetransform) (`KismetMathLibrary.MakeRotator` _returnvalue_2 _returnvalue_3 _returnvalue) (.scale _outinstancetransform)) false false false)
    (`InstancedStaticMeshComponent.UpdateInstanceTransform` (`self.InstancedStaticMesh1`) _index (`KismetMathLibrary.MakeTransform` (.location _outinstancetransform) (`KismetMathLibrary.MakeRotator` (+ _returnvalue_2 180.0) _returnvalue_3 _returnvalue) (.scale _outinstancetransform)) false false false))
  (`AudioComponent.Stop` (`self.AudioCircus`)))

(event `/Game/BPs/Interfaces/BPI_Interactible.Interact`
  (params (Component :type "ActorComponent Object Reference"))
  (bind _instancedstaticmesh (`self.InstancedStaticMesh`))
  (bind _as_gi_main (`self.As GI Main`))
  (bind _cardstable (`/Game/BPs/Game/GI_Main.CardsTable` _as_gi_main))
  (if (`self.CanDrawCard`)
    (set `self.CanDrawCard` false)
    (`/Engine/EditorBlueprintResources/StandardMacros.IsValid` _as_gi_main
      (:`Is Valid`
        (`/Engine/EditorBlueprintResources/StandardMacros.IsValid` _cardstable
          (:`Is Valid`
            (bind _level (`/Game/BPs/Game/GI_Main.GetNextLevel` (`self.As GI Main`)))
            (`|ExecutionSequence`
              (:`then_0`
                (bind _returnvalue (`KismetStringLibrary.Conv_StringToName` (`|GetEnumeratorNameAsString` _level)))
                (bind _returnvalue_2 (`|GetDataTableRow` _cardstable _returnvalue)
                  (:`then`
                    (bind (_level_2 _image _text) (break `/Game/Assets/Cards/Struct_CardsInfo` _returnvalue_2))
                    (`KismetSystemLibrary.LogString` (`KismetTextLibrary.Conv_TextToString` _text))
                    (`/Game/BPs/Game/GI_Main.StartedLevel` (`self.As GI Main`))
                    (bind _returnvalue_3 (`|SpawnActorFromClass` "/Game/BPs/Cards/BP_Card.BP_Card_C" (`KismetMathLibrary.MakeTransform` (.location (`InstancedStaticMeshComponent.GetInstanceTransform` _instancedstaticmesh (- (`InstancedStaticMeshComponent.GetInstanceCount` _instancedstaticmesh) 1) true)) (struct :`Pitch` -90.0) (`self.CardSpawnedScale`)) "Undefined" "MultiplyWithRoot" null null))
                    (`/Game/BPs/Cards/BP_Card.Init` _returnvalue_3 _text _image)
                    (add `/Game/BPs/Cards/BP_Card.ED_OpenRoom` _returnvalue_3 (delegate `proxy_OpenRoom`)))
                  (:`RowNotFound`
                    (`KismetSystemLibrary.LogString` "Row not found")
                    (`KismetSystemLibrary.LogString` (`KismetStringLibrary.Conv_NameToString` _returnvalue)))))
              (:`then_1`
                (if (`|EnumEquality` _level "NewEnumerator1")
                  (`GameplayStatics.PlaySound2D` "/Game/Assets/Sounds/MetaSounds/Voices/MS_CircusStart.MS_CircusStart" 1.0 1.0 0.0 null null)
                  (`AudioComponent.Play` (`self.AudioCircus`) 0.0)))))
          (:`Is Not Valid`
            (`KismetSystemLibrary.LogString` "No data table"))))
      (:`Is Not Valid`
        (`KismetSystemLibrary.LogString` "No GI")))))

(event `proxy_OpenRoom`
  (bind _heterogeneousvolume (`/Game/Assets/Animations/BP_Smoke.HeterogeneousVolume` (`self.SmokeRight`)))
  (bind _heterogeneousvolume_2 (`/Game/Assets/Animations/BP_Smoke.HeterogeneousVolume` (`self.SmokeLeft`)))
  (`MovieSceneSequencePlayer.Play` (`LevelSequenceActor.SequencePlayer` (`self.RoomOpenSequence`)))
  (`HeterogeneousVolumeComponent.SetStartFrame` _heterogeneousvolume_2 0.0)
  (`HeterogeneousVolumeComponent.SetPlaying` _heterogeneousvolume_2 false)
  (`HeterogeneousVolumeComponent.SetStartFrame` _heterogeneousvolume 0.0)
  (`HeterogeneousVolumeComponent.SetPlaying` _heterogeneousvolume false))

(fn `UserConstructionScript`
  (for _index (range (`self.NumCards`))
    (bind _returnvalue (* _index (`self.CardsOffset`)))
    (`InstancedStaticMeshComponent.AddInstance` (`self.InstancedStaticMesh`) (`KismetMathLibrary.MakeTransform` _returnvalue) false)
    (`InstancedStaticMeshComponent.AddInstance` (`self.InstancedStaticMesh1`) (`KismetMathLibrary.MakeTransform` _returnvalue (struct :`Roll` 180.0)) false)))