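; PC_Player is the player controller, handling mouse look and pause input.
; On BeginPlay it adds the IMC_Main Enhanced Input mapping context and caches the game HUD.
; IA_Pause calls the HUD's pause event with its gameplay widget, while IA_Mouse drives yaw and inverted-sign pitch, both scaled by a sensitivity value.
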(event `self.ReceiveBeginPlay`
  (`EnhancedInputSubsystemInterface.AddMappingContext` (subsystem `EnhancedInputLocalPlayerSubsystem`) "/Game/Inputs/IMC_Main.IMC_Main" 0 (struct))
  (bind _ashud_game (cast `/Game/BPs/Game/HUD_Game` (`self.GetHUD`)))
  (set `self.As HUD Game` _ashud_game))

(event `EnhancedInput|/Game/Inputs/Actions/IA_Pause`
  (params (ActionValue :type Boolean) (ElapsedSeconds :type "Float (double-precision)") (TriggeredSeconds :type "Float (double-precision)") (InputAction :type "InputAction Object Reference" :default "/Game/Inputs/Actions/IA_Pause.IA_Pause"))
  (bind _as_hud_game (`self.As HUD Game`))
  (:`Started`
    (`/Game/BPs/Game/HUD_Game.CE_Pause` _as_hud_game (`/Game/BPs/Game/HUD_Game.WBP_Gameplay` _as_hud_game))))

(event `EnhancedInput|/Game/Inputs/Actions/IA_Mouse`
  (params (ActionValue :type "Vector2D Structure") (ElapsedSeconds :type "Float (double-precision)") (TriggeredSeconds :type "Float (double-precision)") (InputAction :type "InputAction Object Reference" :default "/Game/Inputs/Actions/IA_Mouse.IA_Mouse"))
  (bind _returnvalue (/ (`self.Sensibility`) 100.0))
  (:`Triggered`
    (`self.AddYawInput` (* ActionValue_X _returnvalue))
    (`self.AddPitchInput` (- 0.0 (* _returnvalue ActionValue_Y)))))

(fn `UserConstructionScript`)