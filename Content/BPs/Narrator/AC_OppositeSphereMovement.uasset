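; Actor component that keeps its owner on a sphere around a center actor, opposite a target actor.
; Each Tick, once both references are valid, it takes the yaw from the target through the center using Atan2.
; Horizontal distance sets the pitch, from straight up at the center down to level at the sphere radius and beyond.
; The owner is then moved to that point on the sphere's surface.
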(event `self.ReceiveTick`
  (params (DeltaSeconds :type "Float (single-precision)"))
  (bind _returnvalue (- (`Actor.K2_GetActorLocation` (`self.SphereCenter`)) (`Actor.K2_GetActorLocation` (`self.Target`))))
  ; Tick
  (if (`self.AreRefsValid`)
    (`Actor.K2_SetActorLocation` (`self.GetOwner` self) (+ (`Actor.K2_GetActorLocation` (`self.SphereCenter`)) (* (`KismetMathLibrary.GetForwardVector` (`KismetMathLibrary.MakeRotator` (.roll (`KismetMathLibrary.RotatorFromAxisAndAngle` (0.0 0.0 1.0) (`KismetMathLibrary.DegAtan2` (.y _returnvalue) (.x _returnvalue)))) (+ (.pitch (`KismetMathLibrary.RotatorFromAxisAndAngle` (0.0 0.0 1.0) (`KismetMathLibrary.DegAtan2` (.y _returnvalue) (.x _returnvalue)))) (`KismetMathLibrary.FClamp` (`KismetMathLibrary.Lerp` 90.0 0.0 (`self.InverseLerp` (`KismetMathLibrary.VSizeXY` _returnvalue) 0.0 (`self.SphereRadius`))) 0.0 90.0)) (.yaw (`KismetMathLibrary.RotatorFromAxisAndAngle` (0.0 0.0 1.0) (`KismetMathLibrary.DegAtan2` (.y _returnvalue) (.x _returnvalue)))))) (`self.SphereRadius`))) false false)))